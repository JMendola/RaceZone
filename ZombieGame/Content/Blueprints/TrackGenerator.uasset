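; Spline-driven track generator that builds a road with optional left and right guard rails in the construction script.
; It resizes RoadDataArray to match the spline point count, giving each point its own bank, width, thickness and rail toggles.
; BuildTrackElements adds a spline mesh per segment, interpolating roll and scale between neighbouring points, with optional collision and looping.
; An optional debug pass places numbered text labels above each spline point.
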(event EventBeginPlay)

(event Collision|EventActorBeginOverlap
  (params (OtherActor :type Actor%20Object%20Reference)))

(event EventTick
  (params (DeltaSeconds :type Float%20%28single-precision%29)))

(fn ConstructionScript
  (bind _roaddataarray (Variables|Default|GetRoadDataArray))
  (Utilities|FlowControl|Sequence
    (:then_0
      (Variables|Default|SetNumberOfSplinePoints (Spline|GetNumberOfSplinePoints (Variables|Default|GetSpline))))
    (:then_1
      (Math|Integer|CompareInt (Utilities|Array|Length (Variables|Default|GetRoadDataArray)) (Variables|Default|GetNumberOfSplinePoints) :!label _label
        (:>
          (Utilities|Array|RemoveIndex _roaddataarray (Utilities|Array|LastIndex _roaddataarray))
          (goto _label))
        (:<
          (Utilities|Array|Add :TargetArray (Variables|Default|GetRoadDataArray))
          (goto _label))))
    (:then_2
      (for _index (range 0 (- (Variables|Default|GetNumberOfSplinePoints) (Math|Integer|SelectInt 1 2 (Variables|Default|GetLoopingTrack))))
        (Variables|Default|SetCurrentLoopIndex _index)
        (Variables|Default|SetDrawLeftGuardRail (.leftguardrail (Utilities|Array|Get(acopy) (Variables|Default|GetRoadDataArray) (Variables|Default|GetCurrentLoopIndex))))
        (Variables|Default|SetDrawRightGuardRail (.rightguardrail (Utilities|Array|Get(acopy) (Variables|Default|GetRoadDataArray) (Variables|Default|GetCurrentLoopIndex))))
        (Utilities|FlowControl|Sequence
          (:then_0
            (CallFunction|BuildTrackElements (Variables|Default|GetCurrentLoopIndex) (Variables|Default|GetRoadMesh)))
          (:then_1
            (if (Variables|Default|GetDrawLeftGuardRail)
              (CallFunction|BuildTrackElements (Variables|Default|GetCurrentLoopIndex) (Variables|Default|GetLeftGuardMesh))))
          (:then_2
            (if (Variables|Default|GetDrawRightGuardRail)
              (CallFunction|BuildTrackElements (Variables|Default|GetCurrentLoopIndex) (Variables|Default|GetRightGuardMesh)))))))
    (:then_3
      (if (Variables|Default|GetDrawTrackPointNumbers)
        (for _index_2 (range 0 (- (Variables|Default|GetNumberOfSplinePoints) 1))
          (Variables|Default|SetCurrenTrackPoint (Utilities|Text|ToText(Integer) _index_2))
          (bind _returnvalue (AddComponent|AddTextRenderComponent false (Math|Transform|MakeTransform (Math|Vector|MakeVector (.X (Math|Vector|BreakVector (.Location (Spline|GetLocationandTangentatSplinePoint (Variables|Default|GetSpline) _index_2 "Local")))) (.Y (Math|Vector|BreakVector (.Location (Spline|GetLocationandTangentatSplinePoint (Variables|Default|GetSpline) _index_2 "Local")))) (+ (.Z (Math|Vector|BreakVector (.Location (Spline|GetLocationandTangentatSplinePoint (Variables|Default|GetSpline) _index_2 "Local")))) 5e+01)) (Math|Conversions|RotationFromXVector (* (.Tangent (Spline|GetLocationandTangentatSplinePoint (Variables|Default|GetSpline) _index_2 "Local")) -1.0)))))
          (Rendering|Components|TextRender|SetText _returnvalue (Variables|Default|GetCurrenTrackPoint)))))))

(fn BuildTrackElements
  (params (LoopIndex :type Integer) (TrackElementMesh :type Static%20Mesh%20Object%20Reference))
  (LocalVariables|SetLocal_CurrentLoopIndex LoopIndex)
  (LocalVariables|SetLocal_NextLoopIndex (Math|Integer|%(Integer) (+ LoopIndex 1) (Variables|Default|GetNumberOfSplinePoints)))
  (LocalVariables|SetLocal_TrackElementMesh TrackElementMesh)
  (Utilities|FlowControl|Sequence
    (:then_0
      (LocalVariables|SetLocal_StartLocation (.Location (Spline|GetLocationandTangentatSplinePoint (Variables|Default|GetSpline) (LocalVariables|GetLocal_CurrentLoopIndex) "Local")))
      (LocalVariables|SetLocal_StartTangent (.Tangent (Spline|GetLocationandTangentatSplinePoint (Variables|Default|GetSpline) (LocalVariables|GetLocal_CurrentLoopIndex) "Local")))
      (LocalVariables|SetLocal_EndLocation (.Location (Spline|GetLocationandTangentatSplinePoint (Variables|Default|GetSpline) (LocalVariables|GetLocal_NextLoopIndex) "Local")))
      (LocalVariables|SetLocal_EndTangent (.Tangent (Spline|GetLocationandTangentatSplinePoint (Variables|Default|GetSpline) (LocalVariables|GetLocal_NextLoopIndex) "Local")))
      (LocalVariables|SetLocal_StartRoll (.trackbank (Utilities|Array|Get(acopy) (Variables|Default|GetRoadDataArray) (LocalVariables|GetLocal_CurrentLoopIndex))))
      (LocalVariables|SetLocal_StartScale (Math|Vector2D|MakeVector2D (.trackwidth (Utilities|Array|Get(acopy) (Variables|Default|GetRoadDataArray) (LocalVariables|GetLocal_CurrentLoopIndex))) (.trackthinckness (Utilities|Array|Get(acopy) (Variables|Default|GetRoadDataArray) (LocalVariables|GetLocal_CurrentLoopIndex)))))
      (LocalVariables|SetLocal_EndRoll (.trackbank (Utilities|Array|Get(acopy) (Variables|Default|GetRoadDataArray) (LocalVariables|GetLocal_NextLoopIndex))))
      (LocalVariables|SetLocal_EndScale (Math|Vector2D|MakeVector2D (.trackwidth (Utilities|Array|Get(acopy) (Variables|Default|GetRoadDataArray) (LocalVariables|GetLocal_NextLoopIndex))) (.trackthinckness (Utilities|Array|Get(acopy) (Variables|Default|GetRoadDataArray) (LocalVariables|GetLocal_NextLoopIndex))))))
    (:then_1
      (bind _returnvalue (AddComponent|AddSplineMeshComponent false))
      (LocalVariables|SetLocal_CurrentSplineMesh _returnvalue)
      (Components|StaticMesh|SetStaticMesh (LocalVariables|GetLocal_CurrentSplineMesh) (LocalVariables|GetLocal_TrackElementMesh))
      (SplineMesh|SetStartandEnd (LocalVariables|GetLocal_CurrentSplineMesh) (LocalVariables|GetLocal_StartLocation) (LocalVariables|GetLocal_StartTangent) (LocalVariables|GetLocal_EndLocation) (LocalVariables|GetLocal_EndTangent) true :!class /Script/Engine.SplineMeshComponent)
      (Class|SplineMeshComponent|SetStartRoll (LocalVariables|GetLocal_CurrentSplineMesh) (LocalVariables|GetLocal_StartRoll) true)
      (Class|SplineMeshComponent|SetEndRoll (LocalVariables|GetLocal_CurrentSplineMesh) (LocalVariables|GetLocal_EndRoll) true)
      (SplineMesh|SetStartScale (LocalVariables|GetLocal_CurrentSplineMesh) (LocalVariables|GetLocal_StartScale) true :!class /Script/Engine.SplineMeshComponent)
      (SplineMesh|SetEndScale (LocalVariables|GetLocal_CurrentSplineMesh) (LocalVariables|GetLocal_EndScale) true :!class /Script/Engine.SplineMeshComponent)
      (Collision|SetCollisionEnabled (LocalVariables|GetLocal_CurrentSplineMesh) (select (Variables|Default|GetCollisions) "QueryAndPhysics" "NoCollision")))))